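; Actor component that lets its owner interact with BP_InteractableBase actors.
; Tick line-traces forward from slightly above the owner and prints an interact prompt when it hits an interactable.
; TryInteract first scans all interactables for one whose positive proximity radius contains the owner, calling HandleInteract on the first match.
; Failing that, it repeats the forward trace and calls HandleInteract on the hit interactable; Interact is an empty stub.
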(event `self.ReceiveTick`
  (params (DeltaSeconds :type "Float (single-precision)"))
  (bind _returnvalue (`self.GetOwner`))
  (bind _returnvalue_2 (+ (`Actor.K2_GetActorLocation` _returnvalue) (`KismetMathLibrary.MakeVector` 0.0 0.0 50.0)))
  (bind (_outhit _returnvalue_3) (`KismetSystemLibrary.LineTraceSingle` _returnvalue_2 (+ _returnvalue_2 (* (`Actor.GetActorForwardVector` _returnvalue) (`self.InteractionRange`))) "TraceTypeQuery1"))
  (if _returnvalue_3
    (cast `/Game/LD_Gym/Interactables/BP_InteractableBase` (`.HitActor` (`GameplayStatics.BreakHitResult` _outhit)))
    (`KismetSystemLibrary.PrintString` "[ E ]  Interact" true true (struct :`G` 0.66 :`B` 1.0 :`A` 1.0) 0.12 "interactprompt")))

(fn `Interact`)

(fn `TryInteract`
  (bind _returnvalue (`self.GetOwner`))
  (bind _returnvalue_2 (+ (`Actor.K2_GetActorLocation` _returnvalue) (`KismetMathLibrary.MakeVector` 0.0 0.0 50.0)))
  (bind _handled (`self.TryInteractNearby`))
  (if (not _handled)
    (bind (_outhit _returnvalue_3) (`KismetSystemLibrary.LineTraceSingle` _returnvalue_2 (+ _returnvalue_2 (* (`Actor.GetActorForwardVector` _returnvalue) (`self.InteractionRange`))) "TraceTypeQuery1"))
    (if _returnvalue_3
      (bind _asbp_interactable_base (cast `/Game/LD_Gym/Interactables/BP_InteractableBase` (`.HitActor` (`GameplayStatics.BreakHitResult` _outhit))))
      (`/Game/LD_Gym/Interactables/BP_InteractableBase.HandleInteract` _asbp_interactable_base))))

(fn `TryInteractNearby`
  (returns (Handled :type Boolean))
  (bind _outactors (`GameplayStatics.GetAllActorsOfClass` "/Game/LD_Gym/Interactables/BP_InteractableBase.BP_InteractableBase_C"))
  (for _array_element _outactors
    (bind _asbp_interactable_base (cast `/Game/LD_Gym/Interactables/BP_InteractableBase` _array_element))
    (bind _proximityinteractradius (`/Game/LD_Gym/Interactables/BP_InteractableBase.ProximityInteractRadius` _asbp_interactable_base))
    (if (> _proximityinteractradius 0.0)
      (if (<= (`KismetMathLibrary.Vector_Distance` (`Actor.K2_GetActorLocation` (`self.GetOwner`)) (`Actor.K2_GetActorLocation` _array_element)) _proximityinteractradius)
        (`/Game/LD_Gym/Interactables/BP_InteractableBase.HandleInteract` _asbp_interactable_base)
        (return true))))
  (return false))