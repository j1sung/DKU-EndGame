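; BP_SpiritVent is a glowing spirit wisp actor with a matching light, able to burst on overlap or on demand.
; Construction script and BeginPlay push color, motion and fade settings into a dynamic material; BeginPlay also configures the light and trigger.
; Optional overlap activation or TriggerBurst stamps game time into BurstStartTime, leaving burst animation to the material without Tick.
; SetFadeAlpha scales light intensity and material fade, hiding mesh and light at zero.
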(event `self.ReceiveBeginPlay`
  (bind _energycolor (`self.EnergyColor`))
  (bind _spiritlight (`self.SpiritLight`))
  (bind _returnvalue (`PrimitiveComponent.CreateDynamicMaterialInstance` (`self.WispMesh`) 0 null "None"))
  (set `self.MID` _returnvalue)
  (`MaterialInstanceDynamic.SetVectorParameterValue` _returnvalue "EnergyColor" _energycolor)
  (`MaterialInstanceDynamic.SetScalarParameterValue` _returnvalue "BurstAmount" 0.0)
  (`LightComponent.SetLightColor` _spiritlight _energycolor true)
  (`LightComponent.SetIntensity` _spiritlight (`self.LightIntensity`))
  (`PrimitiveComponent.SetCollisionProfileName` (`self.TriggerBox`) "OverlapAllDynamic" true)
  (`MaterialInstanceDynamic.SetScalarParameterValue` _returnvalue "IdleBrightness" (`self.IdleBrightness`))
  (`MaterialInstanceDynamic.SetScalarParameterValue` _returnvalue "RiseSpeed" (`self.RiseSpeed`))
  (`MaterialInstanceDynamic.SetScalarParameterValue` _returnvalue "ShrinkAmount" (`self.ShrinkAmount`))
  (`MaterialInstanceDynamic.SetScalarParameterValue` _returnvalue "SwirlSpeed" (`self.SwirlSpeed`))
  (`MaterialInstanceDynamic.SetScalarParameterValue` _returnvalue "TipFadeStart" (`self.TipFadeStart`))
  (`MaterialInstanceDynamic.SetScalarParameterValue` _returnvalue "TipFadeEnd" (`self.TipFadeEnd`))
  (`MaterialInstanceDynamic.SetScalarParameterValue` _returnvalue "BaseFadeStart" (`self.BaseFadeStart`))
  (`MaterialInstanceDynamic.SetScalarParameterValue` _returnvalue "BaseFadeEnd" (`self.BaseFadeEnd`)))

(event `self.ReceiveActorBeginOverlap`
  (params (OtherActor :type "Actor Object Reference"))
  (if (`self.bActivateOnOverlap`)
    (`MaterialInstanceDynamic.SetScalarParameterValue` (`self.MID`) "BurstStartTime" (`KismetSystemLibrary.GetGameTimeInSeconds`))))

(event `TriggerBurst`
  (`MaterialInstanceDynamic.SetScalarParameterValue` (`self.MID`) "BurstStartTime" (`KismetSystemLibrary.GetGameTimeInSeconds`)))

(fn `SetFadeAlpha`
  (params (Alpha :type "Float (double-precision)"))
  (bind _wispmesh (`self.WispMesh`))
  (bind _spiritlight (`self.SpiritLight`))
  (bind _returnvalue (> Alpha 0.0))
  (`SceneComponent.SetVisibility` _wispmesh _returnvalue false)
  (`SceneComponent.SetVisibility` _spiritlight _returnvalue false)
  (`LightComponent.SetIntensity` _spiritlight (* (`self.LightIntensity`) Alpha))
  (`MeshComponent.SetScalarParameterValueOnMaterials` _wispmesh "FadeAlpha" Alpha))

(fn `UserConstructionScript`
  (bind _returnvalue (`PrimitiveComponent.CreateDynamicMaterialInstance` (`self.WispMesh`) 0 null "None"))
  (set `self.MID` _returnvalue)
  (`MaterialInstanceDynamic.SetVectorParameterValue` _returnvalue "EnergyColor" (`self.EnergyColor`))
  (`MaterialInstanceDynamic.SetScalarParameterValue` _returnvalue "IdleBrightness" (`self.IdleBrightness`))
  (`MaterialInstanceDynamic.SetScalarParameterValue` _returnvalue "RiseSpeed" (`self.RiseSpeed`))
  (`MaterialInstanceDynamic.SetScalarParameterValue` _returnvalue "ShrinkAmount" (`self.ShrinkAmount`))
  (`MaterialInstanceDynamic.SetScalarParameterValue` _returnvalue "SwirlSpeed" (`self.SwirlSpeed`))
  (`MaterialInstanceDynamic.SetScalarParameterValue` _returnvalue "TipFadeStart" (`self.TipFadeStart`))
  (`MaterialInstanceDynamic.SetScalarParameterValue` _returnvalue "TipFadeEnd" (`self.TipFadeEnd`))
  (`MaterialInstanceDynamic.SetScalarParameterValue` _returnvalue "BaseFadeStart" (`self.BaseFadeStart`))
  (`MaterialInstanceDynamic.SetScalarParameterValue` _returnvalue "BaseFadeEnd" (`self.BaseFadeEnd`)))