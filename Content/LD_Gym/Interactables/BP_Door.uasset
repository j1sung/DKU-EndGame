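; Interactable door Blueprint for the level design gym that opens on interaction unless Locked.
; HandleInteract only opens the door, with no toggle to close it.
; SetDoorOpen stores IsOpen, calls OnDoorStateChanged, then snaps DoorMesh vertically between closed and raised positions, without animation or sweep.
; Disconnected leftover nodes include an unused yaw-rotation variant driven by OpenAngle.
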(event `self.HandleInteract`
  (if (not (`self.bLocked`))
    (`self.SetDoorOpen` true)))

(fn `SetDoorOpen`
  (params (bWantOpen :type Boolean))
  (set `self.bIsOpen` bWantOpen)
  (`self.OnDoorStateChanged`)
  (`SceneComponent.K2_SetRelativeLocation` (`self.DoorMesh`) (select `bool` bWantOpen :`false` (`KismetMathLibrary.MakeVector` 0.0) :`true` (`KismetMathLibrary.MakeVector` 0.0 0.0 260.0)) false false))

(fn `UserConstructionScript`)