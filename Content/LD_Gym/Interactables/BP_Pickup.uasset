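; BP_Pickup is a pickup actor that spins around its yaw axis every tick at a constant rate.
; HandleInteract runs Collect, which fires the OnCollected dispatcher and destroys the actor.
; Overlap by any Character destroys the actor directly, bypassing Collect, so OnCollected does not fire on that path.
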(event `self.HandleInteract`
  (`self.Collect`))

(event `self.ReceiveActorBeginOverlap`
  (params (OtherActor :type "Actor Object Reference"))
  (cast `Character` OtherActor)
  (`self.K2_DestroyActor` self))

(event `self.ReceiveTick`
  (params (DeltaSeconds :type "Float (single-precision)"))
  (`self.K2_AddActorLocalRotation` self (`KismetMathLibrary.MakeRotator` 0.0 0.0 (* 120.0 DeltaSeconds)) false false))

(fn `Collect`
  (`self.OnCollected`)
  (`self.K2_DestroyActor` self))

(fn `UserConstructionScript`)