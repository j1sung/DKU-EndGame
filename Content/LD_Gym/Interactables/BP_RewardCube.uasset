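; BP_RewardCube is an interactable pickup in the LD_Gym content that the player collects at close range.
; HandleInteract compares the distance between player pawn 0 and the cube to ProximityInteractRadius.
; Within that radius, it broadcasts the OnCollected dispatcher and destroys the actor.
; BeginPlay, overlap, Tick and the construction script only call their parent versions.
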(event `self.ReceiveBeginPlay`
  (`parent.ReceiveBeginPlay`))

(event `self.ReceiveActorBeginOverlap`
  (params (OtherActor :type "Actor Object Reference"))
  (`parent.ReceiveActorBeginOverlap` OtherActor))

(event `self.ReceiveTick`
  (params (DeltaSeconds :type "Float (single-precision)"))
  (`parent.ReceiveTick` DeltaSeconds))

(event `self.HandleInteract`
  (if (<= (`KismetMathLibrary.Vector_Distance` (`self.K2_GetActorLocation` (`GameplayStatics.GetPlayerPawn` 0)) (`self.K2_GetActorLocation`)) (`self.ProximityInteractRadius`))
    (`self.OnCollected`)
    (`self.K2_DestroyActor`)))

(fn `UserConstructionScript`
  (`parent.UserConstructionScript`))